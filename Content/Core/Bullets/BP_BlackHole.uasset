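; BP_BlackHole is a bullet-folder actor that plays a black hole effect, swallowing the actor it hit.
; On BeginPlay a timeline scales the mesh from its Scale track.
; The same timeline's EaseInOut track pulls a valid HitActor from its start location to the black hole's center while shrinking it to nothing.
; When the timeline finishes, it calls OnBlackHoleAnimationEnded.
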(event `self.ReceiveBeginPlay`
  (bind (_direction _scale _easeinout) (`Timeline|Timeline`)
    (:`Update`
      (`|ExecutionSequence`
        (:`then_0`
          (`SceneComponent.SetWorldScale3D` (`self.Mesh`) (`KismetMathLibrary.Conv_DoubleToVector` (* _scale 10.0))))
        (:`then_1`
          (bind _hitactor (`self.HitActor`)
            (:`then`
              (`|ExecutionSequence`
                (:`then_0`
                  (`self.K2_SetActorLocation` _hitactor (`KismetMathLibrary.VLerp` (`self.HitActorStartLocation`) (`self.K2_GetActorLocation`) _easeinout) false false))
                (:`then_1`
                  (`self.SetActorScale3D` _hitactor (`KismetMathLibrary.Conv_DoubleToVector` (`KismetMathLibrary.Lerp` 1.0 0.0 _easeinout))))))
            (:`else`)))))
    (:`Finished`
      (`self.OnBlackHoleAnimationEnded`))))

(fn `UserConstructionScript`)